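; BP_BallMenu is a Pong-style ball, apparently for the menu, that serves itself in a random direction on BeginPlay.
; Overlaps drive bouncing by rewriting physics velocity: horizontal boundaries flip X, vertical boundaries flip Y and randomly offset X.
; Each bounce plays one of two sounds chosen by a Sound flag.
; Paddle, goal, scoring and game-over functions exist, but the event graph never calls them.
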(event EventBeginPlay
  (CallFunction|ServeBall))

(event Collision|EventActorBeginOverlap
  (params (OtherActor :type Actor%20Object%20Reference))
  ;[1 1 1] Boundry Workings
  (Utilities|Casting|CastToBP_HorizontalBoundry OtherActor
    (:then
      (CallFunction|BounceOffHBoundry)
      (CallFunction|PlayBoundrySound))
    (:CastFailed
      (Utilities|Casting|CastToBP_VerticalBoundry OtherActor)
      (CallFunction|BounceOffVBoundry)
      (CallFunction|PlayBoundrySound))))

(fn ConstructionScript)

(fn BounceOffHBoundry
  (bind _returnvalue (Physics|GetPhysicsLinearVelocity (Variables|Default|GetStaticMesh) "None"))
  (Physics|SetPhysicsLinearVelocity (Variables|Default|GetStaticMesh) (CallFunction|ReverseXVelocity _returnvalue) false "None"))

(fn BounceOffPaddle
  (params (Target :type Primitive%20Component%20Object%20Reference))
  (bind _returnvalue (Physics|GetPhysicsLinearVelocity Target "None"))
  (bind _returnvalue_2 (Physics|GetPhysicsLinearVelocity (Variables|Default|GetStaticMesh) "None"))
  (Physics|SetPhysicsLinearVelocity (Variables|Default|GetStaticMesh) (CallFunction|ReverseYVelocity _returnvalue_2 (CallFunction|PaddleVelocitywithOffset _returnvalue (Variables|Default|GetHit_Offset_Min) (Variables|Default|GetHit_Offset_Max))) false "None"))

(fn ServeBall
  (Physics|SetPhysicsLinearVelocity (Variables|Default|GetStaticMesh) (CallFunction|PropellBall "0, 0, 0" (CallFunction|RandomiseServer) (Variables|Default|GetServe_Offset_Min) (Variables|Default|GetServe_Offset_Max)) false "None"))

(fn HitGoal
  (params (Server :type Float%20%28single-precision%29%20%28by%20ref%29))
  (Transformation|SetActorLocation "0, 0, 0" false false)
  (Physics|SetPhysicsLinearVelocity (Variables|Default|GetStaticMesh) (CallFunction|PropellBall "0, 0, 0" Server (Variables|Default|GetServe_Offset_Min) (Variables|Default|GetServe_Offset_Max)) false "None"))

(fn PropellBall
  (params (In%20Vec :type Vector) (Server :type Float%20%28single-precision%29%20%28by%20ref%29) (OffsetMin :type Float%20%28single-precision%29%20%28by%20ref%29) (OffsetMax :type Float%20%28single-precision%29%20%28by%20ref%29))
  (bind (_x _y _z) (Math|Vector|BreakVector In%20Vec))
  (return (Math|Vector|MakeVector (+ _x (Math|Random|RandomFloatinRange OffsetMin OffsetMax)) Server _z)))

(fn RandomiseServer
  (return (Math|Float|SelectFloat (Variables|Default|GetServe_R) (Variables|Default|GetServe_L) (Math|Random|RandomBool))))

(fn ReverseXVelocity
  (params (InVec :type Vector))
  (bind (_x _y _z) (Math|Vector|BreakVector InVec))
  (return (Math|Vector|MakeVector (* _x (Variables|Default|GetReverse_Velocity)) _y _z)))

(fn ReverseYVelocity
  (params (InVec :type Vector) (NewParam :type Float%20%28single-precision%29%20%28by%20ref%29))
  (bind (_x _y _z) (Math|Vector|BreakVector InVec))
  (return (Math|Vector|MakeVector NewParam (* _y (Variables|Default|GetReverse_Velocity)) _z)))

(fn PaddleVelocitywithOffset
  (params (InVec :type Vector) (OffsetMin :type Float%20%28single-precision%29) (OffsetMax :type Float%20%28single-precision%29))
  (return (+ (.X (Math|Vector|BreakVector InVec)) (Math|Random|RandomFloatinRange OffsetMin OffsetMax))))

(fn IncreaseLPlayerScore
  (bind _output_get (Variables|Default|SetLPlayer_Score (+ (Variables|Default|GetLPlayer_Score) 1)))
  (CallFunction|UpdateScoreBoard (Variables|Default|GetL_Scoreboard) _output_get))

(fn UpdateScoreBoard
  (params (Tag :type Name%20%28by%20ref%29) (Player :type Integer%20%28by%20ref%29))
  (bind _outactors (Actor|GetAllActorsOfClass "/Script/Engine.TextRenderActor"))
  (for _array_element _outactors
    (if (Components|ComponentHasTag (Variables|/Script/Engine.TextRenderActor|GetTextRender _array_element) Tag)
      (Rendering|Components|TextRender|SetText (Variables|/Script/Engine.TextRenderActor|GetTextRender _array_element) (Utilities|Text|ToText(Integer) Player)))))

(fn IsWinner?
  (params (Player%20Score%20 :type Integer%20%28by%20ref%29) (Player%20Win%20Message :type String%20%28by%20ref%29) (Server :type Float%20%28single-precision%29%20%28by%20ref%29))
  (if (> Player%20Score%20 (- (Variables|Default|GetWinning_Score) 1))
    (Development|PrintString Player%20Win%20Message)
    (Variables|Default|SetbGameOver true)
    (CallFunction|GameOver?)
    (else
      (CallFunction|HitGoal Server))))

(fn IncreaseRPlayerScore
  (bind _output_get (Variables|Default|SetRPlayer_Score (+ (Variables|Default|GetRPlayer_Score) 1)))
  (CallFunction|UpdateScoreBoard (Variables|Default|GetR_Scoreboard) _output_get))

(fn GameOver?
  (if (Variables|Default|GetbGameOver)
    (Physics|SetPhysicsLinearVelocity (Variables|Default|GetStaticMesh) "0, 0, 0" false "None")
    (Transformation|SetActorLocation "0, 0, 0" false false)))

(fn PlayBoundrySound
  (if (Variables|Default|GetSound)
    (Audio|PlaySoundatLocation "/Game/Audio/Low/S_ballCollision.S_ballCollision" "0, 0, 0" "0, 0, 0" 1.0 1.0 0.0 0 0 0)
    (else
      (Audio|PlaySoundatLocation "/Game/Audio/High/ping_pong_8bit_plop.ping_pong_8bit_plop" "0, 0, 0" "0, 0, 0" 1.0 1.0 0.0 0 0 0))))

(fn PlayPaddleSound
  (if (Variables|Default|GetSound)
    (Audio|PlaySoundatLocation "/Game/Audio/Low/S_ballCollision.S_ballCollision" "0, 0, 0" "0, 0, 0" 1.0 1.0 0.0 0 0 0)
    (else
      (Audio|PlaySoundatLocation "/Game/Audio/High/ping_pong_8bit_beeep.ping_pong_8bit_beeep" "0, 0, 0" "0, 0, 0" 1.0 1.0 0.0 0 0 0))))

(fn PlayGoalSound
  (if (Variables|Default|GetSound)
    (Audio|PlaySoundatLocation "/Game/Audio/Low/S_ballGoal.S_ballGoal" "0, 0, 0" "0, 0, 0" 1.0 1.0 0.0 0 0 0)
    (else
      (Audio|PlaySoundatLocation "/Game/Audio/High/ping_pong_8bit_peeeeeep.ping_pong_8bit_peeeeeep" "0, 0, 0" "0, 0, 0" 1.0 1.0 0.0 0 0 0))))

(fn BounceOffVBoundry
  (bind _returnvalue (Physics|GetPhysicsLinearVelocity (Variables|Default|GetStaticMesh) "None"))
  (bind _returnvalue_2 (Physics|GetPhysicsLinearVelocity (Variables|Default|GetStaticMesh) "None"))
  (Physics|SetPhysicsLinearVelocity (Variables|Default|GetStaticMesh) (CallFunction|ReverseYVelocity _returnvalue_2 (CallFunction|PaddleVelocitywithOffset _returnvalue (Variables|Default|GetHit_Offset_Min) (Variables|Default|GetHit_Offset_Max))) false "None"))
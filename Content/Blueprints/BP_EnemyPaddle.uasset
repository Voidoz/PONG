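; AI-controlled enemy paddle for a ball-and-paddle game, moving along X with physics.
; Each tick, for every BP_Ball, it clamps itself between Top and Bottom, zeroing velocity at the limits, then runs AI.
; The default AI applies clamped force toward the ball's X position.
; AIType 1, read from the player's Vars character, is meant for trajectory prediction but applies zero impulse, leaving the two-trace prediction helper disconnected.
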(event Custom|Delay
  (params (Duration :type Float%20%28single-precision%29))
  (Utilities|FlowControl|Delay Duration))

(event EventBeginPlay
  (if (and (Math|Float|NearlyEqual(Float) (Variables|Default|GetBall_X_Axis) 0.0 2.5e+02) (< (Variables|Default|GetBall_Y_Axis) 0.0))
    _))

(event Collision|EventActorBeginOverlap
  (params (OtherActor :type Actor%20Object%20Reference)))

(event EventTick
  (params (DeltaSeconds :type Float%20%28single-precision%29))
  (bind _outactors (Actor|GetAllActorsOfClass "/Game/Blueprints/BP_Ball.BP_Ball_C"))
  (for _array_element _outactors
    (bind _asbp_ball (Utilities|Casting|CastToBP_Ball _array_element))
    (CallFunction|EnforceBounds)
    (CallFunction|AI _asbp_ball)))

(fn ConstructionScript)

(fn EnforceBounds
  (bind _returnvalue (Transformation|GetActorLocation))
  (bind _returnvalue_2 (Transformation|GetActorLocation))
  (bind (_x _y _z) (Math|Vector|BreakVector _returnvalue))
  (bind (_x_2 _y_2 _z_2) (Math|Vector|BreakVector _returnvalue_2))
  (if (> (.X (Math|Vector|BreakVector (Transformation|GetActorLocation))) (Variables|Default|GetTop))
    (Transformation|SetActorLocation (Math|Vector|MakeVector (- (Variables|Default|GetTop) (Variables|Default|GetResistance)) _y_2 _z_2) false false)
    (Physics|SetPhysicsLinearVelocity (Variables|Default|GetAI_Paddle_Mesh) "0, 0, 0" false "None")
    (elif (< (.X (Math|Vector|BreakVector (Transformation|GetActorLocation))) (Variables|Default|GetBottom))
      (Transformation|SetActorLocation (Math|Vector|MakeVector (+ (Variables|Default|GetBottom) (Variables|Default|GetResistance)) _y _z) false false)
      (Physics|SetPhysicsLinearVelocity (Variables|Default|GetAI_Paddle_Mesh) "0, 0, 0" false "None")
      (else
        (return)))))

(fn PredictBallTrajectory
  (params (InputPin :type Actor%20Object%20Reference))
  (bind _array (Utilities|Array|MakeArray "ObjectTypeQuery2"))
  (bind (_outhit _outpathpositions _outlasttracedestination _returnvalue) (Class|GameplayStatics|BlueprintPredictProjectilePathbyObjectType (Transformation|GetActorLocation InputPin) (Transformation|GetVelocity InputPin) true 0.0 _array true (Utilities|Array|MakeArray (Variables|Default|GetBP_L_Goal) (Variables|Default|GetBP_R_Goal) self) "None"))
  (if _returnvalue
    (bind _outlasttracedestination_2 (Class|GameplayStatics|BlueprintPredictProjectilePathbyObjectType _outlasttracedestination (Transformation|GetVelocity InputPin) true 0.0 _array true 0 "None"))
    (return _outlasttracedestination_2)
    (else
      (return _outlasttracedestination))))

(fn AI
  (params (Target :type Actor%20Object%20Reference))
  (bind _returnvalue (Transformation|GetActorLocation Target))
  (bind (_x _y) (Math|Vector|BreakVector _returnvalue))
  (Variables|Default|SetBall_X_Axis _x)
  (Variables|Default|SetBall_Y_Axis _y)
  (if (== (Variables|/Game/Blueprints/Vars.Vars_C|GetAI_Type (CallFunction|GlobalVars)) 1)
    ;[1 1 1] Use Trajectory
    (Physics|AddImpulse (Variables|Default|GetAI_Paddle_Mesh) "0, 0, 0" "None" false)
    (else
      ;[1 1 1] Use Location
      (Physics|AddForce (Variables|Default|GetAI_Paddle_Mesh) (* (Math|Vector|MakeVector (Math|Float|Clamp(Float) (- (.X (Math|Vector|BreakVector (Transformation|GetActorLocation Target))) (.X (Math|Vector|BreakVector (Transformation|GetActorLocation)))) -1e+01 1e+01) 0.0 0.0) (Variables|Default|GetAI_Paddle_Speed_1)) "None" false))))

(fn GetActorLoc
  (params (InVec :type Vector))
  (if (> (.X (Math|Vector|BreakVector InVec)) (.X (Math|Vector|BreakVector (Transformation|GetActorLocation))))
    (return (- (Transformation|GetActorLocation) 175.0))
    (elif (< (.X (Math|Vector|BreakVector InVec)) (.X (Math|Vector|BreakVector (Transformation|GetActorLocation))))
      (return (- (Transformation|GetActorLocation) -175.0))
      (else
        (return "0, 0, 0")))))

(fn GlobalVars
  (bind _asvars (Utilities|Casting|CastToVars (Game|GetPlayerCharacter 0)))
  (return _asvars))
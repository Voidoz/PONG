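; Pong ball that serves itself, handles bounces and scoring, and restarts the match.
; Overlaps flip physics velocity at boundaries and paddles, with paddle X velocity plus random offset steering the rebound.
; Goals update tagged TextRender scoreboards, then re-serve or, at the winning score, print the winner and reload the single- or multiplayer level after a delay, chosen by BP_Paddle_L's presence.
; Collision sounds follow audio settings on the Vars player character.
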(event Custom|RestartGame
  (params (Duration :type Float%20%28single-precision%29%20%28by%20ref%29) (LevelName :type Name))
  (Utilities|FlowControl|Delay Duration)
  (Game|OpenLevel(byName) LevelName))

(event EventBeginPlay
  (CallFunction|ServeBall))

(event Collision|EventActorBeginOverlap
  (params (OtherActor :type Actor%20Object%20Reference))
  ;[1 1 1] Boundry Workings
  (Utilities|Casting|CastToBP_HorizontalBoundry OtherActor
    (:then
      (CallFunction|BounceOffBoundry)
      (CallFunction|PlayBoundrySound))
    (:CastFailed
      ;[1 1 1] Goal Workings
      (Utilities|Casting|CastToBP_L_Goal OtherActor
        (:then
          (CallFunction|IncreaseRPlayerScore)
          (CallFunction|IsWinner? (Variables|Default|GetRPlayer_Score) (Variables|Default|GetR_Wins) (Variables|Default|GetServe_R))
          (CallFunction|PlayGoalSound))
        (:CastFailed
          (Utilities|Casting|CastToBP_R_Goal OtherActor
            (:then
              (CallFunction|IncreaseLPlayerScore)
              (CallFunction|IsWinner? (Variables|Default|GetLPlayer_Score) (Variables|Default|GetL_Wins) (Variables|Default|GetServe_L))
              (CallFunction|PlayGoalSound))
            (:CastFailed
              ;[1 1 1] Paddle Workings
              (bind _asbp_paddle_r (Utilities|Casting|CastToBP_Paddle_R OtherActor)
                (:then
                  (CallFunction|BounceOffPaddle (Variables|/Game/Blueprints/BP_Paddle_R.BP_Paddle_R_C|GetPaddle_Mesh_R _asbp_paddle_r))
                  (CallFunction|PlayPaddleSound))
                (:CastFailed
                  (bind _asbp_enemy_paddle (Utilities|Casting|CastToBP_EnemyPaddle OtherActor)
                    (:then
                      (CallFunction|BounceOffPaddle (Variables|/Game/Blueprints/BP_EnemyPaddle.BP_EnemyPaddle_C|GetAI_Paddle_Mesh _asbp_enemy_paddle))
                      (CallFunction|PlayPaddleSound))
                    (:CastFailed
                      (bind _asbp_paddle_l (Utilities|Casting|CastToBP_Paddle_L OtherActor))
                      (CallFunction|BounceOffPaddle (Variables|/Game/Blueprints/BP_Paddle_L.BP_Paddle_L_C|GetPaddle_Mesh_L _asbp_paddle_l))
                      (CallFunction|PlayPaddleSound))))))))))))

(fn ConstructionScript)

(fn BounceOffBoundry
  (bind _returnvalue (Physics|GetPhysicsLinearVelocity (Variables|Default|GetStaticMesh) "None"))
  (Physics|SetPhysicsLinearVelocity (Variables|Default|GetStaticMesh) (CallFunction|ReverseXVelocity _returnvalue) false "None"))

(fn BounceOffPaddle
  (params (Target :type Primitive%20Component%20Object%20Reference))
  (bind _returnvalue (Physics|GetPhysicsLinearVelocity Target "None"))
  (bind _returnvalue_2 (Physics|GetPhysicsLinearVelocity (Variables|Default|GetStaticMesh) "None"))
  (Physics|SetPhysicsLinearVelocity (Variables|Default|GetStaticMesh) (CallFunction|ReverseYVelocity _returnvalue_2 (CallFunction|PaddleVelocitywithOffset _returnvalue (Variables|Default|GetHit_Offset_Min) (Variables|Default|GetHit_Offset_Max))) false "None"))

(fn ServeBall
  (Physics|SetPhysicsLinearVelocity (Variables|Default|GetStaticMesh) (CallFunction|PropellBall "0, 0, 0" (CallFunction|RandomiseServer) (Variables|Default|GetServe_Offset_Min) (Variables|Default|GetServe_Offset_Max)) false "None"))

(fn HitGoal
  (params (Server :type Float%20%28single-precision%29%20%28by%20ref%29))
  (Transformation|SetActorLocation "0, 0, 0" false false)
  (Physics|SetPhysicsLinearVelocity (Variables|Default|GetStaticMesh) (CallFunction|PropellBall "0, 0, 0" Server (Variables|Default|GetServe_Offset_Min) (Variables|Default|GetServe_Offset_Max)) false "None"))

(fn PropellBall
  (params (In%20Vec :type Vector) (Server :type Float%20%28single-precision%29%20%28by%20ref%29) (OffsetMin :type Float%20%28single-precision%29%20%28by%20ref%29) (OffsetMax :type Float%20%28single-precision%29%20%28by%20ref%29))
  (bind (_x _y _z) (Math|Vector|BreakVector In%20Vec))
  (return (Math|Vector|MakeVector (+ _x (Math|Random|RandomFloatinRange OffsetMin OffsetMax)) Server _z)))

(fn RandomiseServer
  (return (Math|Float|SelectFloat (Variables|Default|GetServe_R) (Variables|Default|GetServe_L) (Math|Random|RandomBool))))

(fn ReverseXVelocity
  (params (InVec :type Vector))
  (bind (_x _y _z) (Math|Vector|BreakVector InVec))
  (return (Math|Vector|MakeVector (* _x (Variables|Default|GetReverse_Velocity)) _y _z)))

(fn ReverseYVelocity
  (params (InVec :type Vector) (XVelocity :type Float%20%28single-precision%29%20%28by%20ref%29))
  (bind (_x _y _z) (Math|Vector|BreakVector InVec))
  (return (Math|Vector|MakeVector XVelocity (* _y (Variables|Default|GetReverse_Velocity)) _z)))

(fn PaddleVelocitywithOffset
  (params (InVec :type Vector) (OffsetMin :type Float%20%28single-precision%29) (OffsetMax :type Float%20%28single-precision%29))
  (return (+ (.X (Math|Vector|BreakVector InVec)) (Math|Random|RandomFloatinRange OffsetMin OffsetMax))))

(fn IncreaseLPlayerScore
  (bind _output_get (Variables|Default|SetLPlayer_Score (+ (Variables|Default|GetLPlayer_Score) 1)))
  (CallFunction|UpdateScoreBoard (Variables|Default|GetL_Scoreboard) _output_get))

(fn UpdateScoreBoard
  (params (Tag :type Name%20%28by%20ref%29) (Player :type Integer%20%28by%20ref%29))
  (bind _outactors (Actor|GetAllActorsOfClass "/Script/Engine.TextRenderActor"))
  (for _array_element _outactors
    (if (Components|ComponentHasTag (Variables|/Script/Engine.TextRenderActor|GetTextRender _array_element) Tag)
      (Rendering|Components|TextRender|SetText (Variables|/Script/Engine.TextRenderActor|GetTextRender _array_element) (Utilities|Text|ToText(Integer) Player)))))

(fn IsWinner?
  (params (Player%20Score%20 :type Integer%20%28by%20ref%29) (Player%20Win%20Message :type String%20%28by%20ref%29) (Server :type Float%20%28single-precision%29%20%28by%20ref%29))
  (if (> Player%20Score%20 (- (Variables|Default|GetWinning_Score) 1))
    (Development|PrintString Player%20Win%20Message)
    (Variables|Default|SetbGameOver true)
    (CallFunction|GameOver?)
    (else
      (CallFunction|HitGoal Server))))

(fn IncreaseRPlayerScore
  (bind _output_get (Variables|Default|SetRPlayer_Score (+ (Variables|Default|GetRPlayer_Score) 1)))
  (CallFunction|UpdateScoreBoard (Variables|Default|GetR_Scoreboard) _output_get))

(fn GameOver?
  (if (Variables|Default|GetbGameOver)
    (bind _outactors (Actor|GetAllActorsOfClass "/Game/Blueprints/BP_Paddle_L.BP_Paddle_L_C"))
    (if (> (Utilities|Array|Length _outactors) 0)
      (Physics|SetPhysicsLinearVelocity (Variables|Default|GetStaticMesh) "0, 0, 0" false "None")
      (Transformation|SetActorLocation "0, 0, 0" false false)
      (CallFunction|RestartGame (Variables|Default|GetRestart_Delay) (Variables|Default|GetSingleplayer_Level))
      (else
        (Physics|SetPhysicsLinearVelocity (Variables|Default|GetStaticMesh) "0, 0, 0" false "None")
        (Transformation|SetActorLocation "0, 0, 0" false false)
        (CallFunction|RestartGame (Variables|Default|GetRestart_Delay) (Variables|Default|GetMultiplayer_Level))))))

(fn PlayBoundrySound
  (if (== (Variables|/Game/Blueprints/Vars.Vars_C|GetBoundry_Audio (CallFunction|GlobalVars)) 0)
    (Audio|PlaySoundatLocation "/Game/Audio/Low/S_ballCollision.S_ballCollision" "0, 0, 0" "0, 0, 0" 1.0 1.0 0.0 0 0 0)
    (else
      (Audio|PlaySoundatLocation "/Game/Audio/High/ping_pong_8bit_plop.ping_pong_8bit_plop" "0, 0, 0" "0, 0, 0" 1.0 1.0 0.0 0 0 0))))

(fn PlayPaddleSound
  (if (== (Variables|/Game/Blueprints/Vars.Vars_C|GetPaddle_Audio (CallFunction|GlobalVars)) 0)
    (Audio|PlaySoundatLocation "/Game/Audio/Low/S_ballCollision.S_ballCollision" "0, 0, 0" "0, 0, 0" 1.0 1.0 0.0 0 0 0)
    (else
      (Audio|PlaySoundatLocation "/Game/Audio/High/ping_pong_8bit_beeep.ping_pong_8bit_beeep" "0, 0, 0" "0, 0, 0" 1.0 1.0 0.0 0 0 0))))

(fn PlayGoalSound
  (if (== (Variables|/Game/Blueprints/Vars.Vars_C|GetGoal_Audio (CallFunction|GlobalVars)) 0)
    (Audio|PlaySoundatLocation "/Game/Audio/Low/S_ballGoal.S_ballGoal" "0, 0, 0" "0, 0, 0" 1.0 1.0 0.0 0 0 0)
    (else
      (Audio|PlaySoundatLocation "/Game/Audio/High/ping_pong_8bit_peeeeeep.ping_pong_8bit_peeeeeep" "0, 0, 0" "0, 0, 0" 1.0 1.0 0.0 0 0 0))))

(fn GlobalVars
  (bind _asvars (Utilities|Casting|CastToVars (Game|GetPlayerCharacter 0)))
  (return _asvars))